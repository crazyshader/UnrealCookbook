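; Demo Blueprint that exercises wildcard-parameter library functions, one for a custom struct and one for an array, triggered by keys 1 and 2.
; Key 1 passes a freshly made BPTest struct to ShowStructFields.
; Key 2 averages the Age property across MyStructArray by property name and prints the formatted result as both text and string.
; A second ShowStructFields call on the first array element is left unconnected.
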(event `Key|One`
  (params (Key :type "Key Structure"))
  ;[1 1 1] CustomStructureParam Function
  (:`Pressed`
    (`BlueprintWildcardLibrary.ShowStructFields` (make `/Game/BlueprintWildcardDemo/BP_Test` false))))

(event `Key|Two`
  (params (Key :type "Key Structure"))
  (bind _mystructarray (`self.MyStructArray`))
  (bind _result (`|FormatText` "Average age of {0} = {1}" (`KismetArrayLibrary.Array_Length` _mystructarray) (`BlueprintWildcardLibrary.Array_NumericPropertyAverage` _mystructarray "Age")))
  ;[1 1 1] ArrayParm Function
  (:`Pressed`
    (`KismetSystemLibrary.PrintText` _result)
    (`KismetSystemLibrary.PrintString` (`KismetTextLibrary.Conv_TextToString` _result))))

(fn `UserConstructionScript`)